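; BP_Eye is a horror eye enemy that roams between random TargetPoints and can kill the player in Panic difficulty.
; A slowed Tick alternates random rotation offsets and a reset through nested FlipFlops, with a Timeline easing the mesh twitch.
; Box overlap kills directly, while capsule overlap requires a line-of-sight trace.
; After a kill or 34-second lifetime, it calls CallDeathPlayer, plays a sound and destroys itself.
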(event OnComponentBeginOverlap(Capsule)
  (params (OverlappedComponent :type Primitive%20Component%20Object%20Reference) (OtherActor :type Actor%20Object%20Reference) (OtherComp :type Primitive%20Component%20Object%20Reference) (OtherBodyIndex :type Integer) (bFromSweep :type Boolean) (SweepResult :type Hit%20Result%20Structure%20%28by%20ref%29))
  (bind _asplayer_character (Utilities|Casting|CastToPlayerCharacter OtherActor))
  (Variables|Default|SetPlayerCharacter _asplayer_character)
  (bind _asplayer_game_instance (Utilities|Casting|CastToPlayerGameInstance (Game|GetGameInstance)))
  (switch Utilities|FlowControl|Switch|SwitchonComplexety (Variables|/Game/Blueprints/Player/PlayerGameInstance.PlayerGameInstance_C|GetGameComplexetty _asplayer_game_instance)
    (:NewEnumerator2
      (CallFunction|Death))))

(event OnComponentBeginOverlap(Box)
  (params (OverlappedComponent :type Primitive%20Component%20Object%20Reference) (OtherActor :type Actor%20Object%20Reference) (OtherComp :type Primitive%20Component%20Object%20Reference) (OtherBodyIndex :type Integer) (bFromSweep :type Boolean) (SweepResult :type Hit%20Result%20Structure%20%28by%20ref%29))
  (bind _asplayer_character (Utilities|Casting|CastToPlayerCharacter OtherActor))
  (Variables|Default|SetPlayerCharacter _asplayer_character)
  (if (not (Variables|/Game/Blueprints/Player/Character/PlayerCharacter.PlayerCharacter_C|GetDeath1 _asplayer_character))
    (bind _asplayer_game_instance (Utilities|Casting|CastToPlayerGameInstance (Game|GetGameInstance)))
    (switch Utilities|FlowControl|Switch|SwitchonComplexety (Variables|/Game/Blueprints/Player/PlayerGameInstance.PlayerGameInstance_C|GetGameComplexetty _asplayer_game_instance)
      (:NewEnumerator2
        (CallFunction|DeathPlayerBox)))))

(event Custom|SetRelativeTransform
  (params (New%20Rotation%20X%20%28Roll%29 :type Float%20%28single-precision%29) (New%20Rotation%20Y%20%28Pitch%29 :type Float%20%28single-precision%29) (New%20Rotation%20Z%20%28Yaw%29 :type Float%20%28single-precision%29))
  (bind _staticmesh (Variables|Default|GetStaticMesh))
  (bind _relativerotation (Variables|/Script/Engine.SceneComponent|GetRelativeRotation _staticmesh))
  (Variables|Default|SetNew%20Rotation%20X%20%28Roll%29 New%20Rotation%20X%20%28Roll%29)
  (Variables|Default|SetNew%20Rotation%20Y%20%28Pitch%29 New%20Rotation%20Y%20%28Pitch%29)
  (Variables|Default|SetNew%20Rotation%20Z%20%28Yaw%29 New%20Rotation%20Z%20%28Yaw%29)
  (Variables|Default|SetRelative%20Rotation%20X%20%28Roll%29 (.roll _relativerotation))
  (Variables|Default|SetRelative%20Rotation%20Y%20%28Pitch%29 (.pitch _relativerotation))
  (Variables|Default|SetRelative%20Rotation%20Z%20%28Yaw%29 (.yaw _relativerotation))
  (bind _newtrack_0 (Timeline|Timeline PlayFromStart)
    (:Update
      (Transformation|SetRelativeRotation _staticmesh (Math|Rotator|MakeRotator (Math|Float|Lerp (Variables|Default|GetRelative%20Rotation%20X%20%28Roll%29) (Variables|Default|GetNew%20Rotation%20X%20%28Roll%29) _newtrack_0) (Math|Float|Lerp (Variables|Default|GetRelative%20Rotation%20Y%20%28Pitch%29) (Variables|Default|GetNew%20Rotation%20Y%20%28Pitch%29) _newtrack_0) (Math|Float|Lerp (Variables|Default|GetRelative%20Rotation%20Z%20%28Yaw%29) (Variables|Default|GetNew%20Rotation%20Z%20%28Yaw%29) _newtrack_0)) true false))))

(event Custom|Death
  (bind _playercharacter (Variables|Default|GetPlayerCharacter))
  (if (not (Variables|/Game/Blueprints/Player/Character/PlayerCharacter.PlayerCharacter_C|GetDeath1 _playercharacter))
    (bind (_outhit _returnvalue) (Collision|LineTraceByChannel (Transformation|GetWorldLocation (Variables|Default|GetPoint)) (Transformation|GetWorldLocation (Variables|/Game/Blueprints/Player/Character/PlayerCharacter.PlayerCharacter_C|GetToPoint _playercharacter)) "TraceTypeQuery2" false 0 "None"))
    (if _returnvalue
      (Utilities|Casting|CastToPlayerCharacter (.HitActor (Collision|BreakHitResult _outhit)))
      (bind _asplayer_game_instance (Utilities|Casting|CastToPlayerGameInstance (Game|GetGameInstance)))
      (Default|Death (Variables|Default|GetPlayerCharacter) (Variables|/Game/Blueprints/Player/PlayerGameInstance.PlayerGameInstance_C|GetGameplayType _asplayer_game_instance) true)
      (Default|CallDeathPlayer)
      (CallFunction|PlaySound)
      (Actor|DestroyActor))))

(event Custom|Eye
  (bind _outactors (Actor|GetAllActorsOfClass "/Script/Engine.TargetPoint"))
  (AI|AIMoveTo self "0, 0, 0" (.OutItem (Utilities|Array|Random _outactors)) 25.0 false
    (:then
      (Utilities|FlowControl|DoOnce false
        (:Completed
          (Utilities|FlowControl|Delay 34.0)
          (Default|CallDeathPlayer)
          (CallFunction|PlaySound)
          (Actor|DestroyActor))))
    (:OnSuccess
      (CallFunction|Eye :!label _label))
    (:OnFail
      (goto _label))))

(event Custom|PlaySound
  (Audio|SpawnSoundatLocation "/Game/Blueprints/Sounds/67df2ab96dead2d.67df2ab96dead2d" (Transformation|GetActorLocation) "0, 0, 0" 1.0 1.0 0.0 "/Game/Sound/BoomBox/BoomBox.BoomBox" 0))

(event Custom|DeathPlayerBox
  (bind _asplayer_game_instance (Utilities|Casting|CastToPlayerGameInstance (Game|GetGameInstance)))
  (Default|Death (Variables|Default|GetPlayerCharacter) (Variables|/Game/Blueprints/Player/PlayerGameInstance.PlayerGameInstance_C|GetGameplayType _asplayer_game_instance) true)
  (Default|CallDeathPlayer)
  (CallFunction|PlaySound)
  (Actor|DestroyActor))

(event EventBeginPlay
  (Actor|Tick|SetActorTickInterval 0.5)
  (bind _outactors (Actor|GetAllActorsOfClass "/Script/Engine.TargetPoint"))
  (AI|AIMoveTo self "0, 0, 0" (.OutItem (Utilities|Array|Random _outactors)) 25.0 false
    (:then
      (Utilities|FlowControl|DoOnce false
        (:Completed
          (Utilities|FlowControl|Delay 34.0)
          (Default|CallDeathPlayer)
          (CallFunction|PlaySound)
          (Actor|DestroyActor))))
    (:OnSuccess
      (CallFunction|Eye :!label _label))
    (:OnFail
      (goto _label))))

(event EventTick
  (params (DeltaSeconds :type Float%20%28single-precision%29))
  (bind _returnvalue (Math|Random|RandomFloatinRange 1.0 2e+01))
  (bind _returnvalue_2 (Math|Random|RandomFloatinRange 1.0 2e+01))
  (bind _staticmesh (Variables|Default|GetStaticMesh))
  (bind _staticmesh_2 (Variables|Default|GetStaticMesh))
  (bind _relativerotation (Variables|/Script/Engine.SceneComponent|GetRelativeRotation _staticmesh))
  (bind _relativerotation_2 (Variables|/Script/Engine.SceneComponent|GetRelativeRotation _staticmesh_2))
  (Utilities|FlowControl|FlipFlop
    (:A
      (CallFunction|SetRelativeTransform (+ (.roll _relativerotation) _returnvalue_2) (+ (.pitch _relativerotation) _returnvalue_2) (+ (.yaw _relativerotation) _returnvalue_2)))
    (:B
      (Utilities|FlowControl|FlipFlop
        (:A
          (CallFunction|SetRelativeTransform (- (.roll _relativerotation_2) _returnvalue) (- (.pitch _relativerotation_2) _returnvalue) (- (.yaw _relativerotation_2) _returnvalue)))
        (:B
          (CallFunction|SetRelativeTransform 115.0 0.0 0.0))))))

(fn ConstructionScript)

(fn RunMulticast)