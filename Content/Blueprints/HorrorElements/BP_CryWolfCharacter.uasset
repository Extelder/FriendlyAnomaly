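; Horror-element character that rushes the nearest living player and plays a very loud sound on reaching them.
; On BeginPlay it scans all player characters, skips those flagged Death1, and targets the closest with AIMoveTo.
; A successful move calls RunMulticast to play the attenuated sound at its location, then destroys the actor.
; It also destroys itself when no target exists or after a short timeout from starting the move.
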(event Custom|RunMulticast
  (Audio|PlaySoundatLocation "/Game/Blueprints/Sounds/67df2ab96dead2d.67df2ab96dead2d" (Transformation|GetActorLocation) "0, 0, 0" 3e+01 1.0 0.0 "/Game/Sound/SoundAttenuation/AnomalySpeaker.AnomalySpeaker" 0 0 0))

(event EventBeginPlay
  (bind _outactors (Actor|GetAllActorsOfClass "/Game/Blueprints/Player/Character/PlayerCharacter.PlayerCharacter_C"))
  (for _array_element _outactors
    (if (not (Variables|/Game/Blueprints/Player/Character/PlayerCharacter.PlayerCharacter_C|GetDeath1 _array_element))
      (Utilities|IsValid (Variables|Default|GetPlayerCharacter)
        (:Is%20Valid
          (if (< (Transformation|GetDistanceTo _array_element) (Variables|Default|GetDistance))
            (Variables|Default|SetPlayerCharacter _array_element :!label _label)
            (Variables|Default|SetDistance (Transformation|GetDistanceTo _array_element))))
        (:Is%20Not%20Valid
          (goto _label)))))
  (Utilities|IsValid (Variables|Default|GetPlayerCharacter)
    (:Is%20Valid
      (AI|AIMoveTo self "0, 0, 0" (Variables|Default|GetPlayerCharacter) 5.0 false
        (:then
          (Utilities|FlowControl|Delay 8.0))
        (:OnSuccess
          (CallFunction|RunMulticast)))
      (Actor|DestroyActor))
    (:Is%20Not%20Valid
      (Actor|DestroyActor))))

(fn ConstructionScript)