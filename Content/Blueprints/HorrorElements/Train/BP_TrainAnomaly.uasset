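; BP_TrainAnomaly is a horror train anomaly that rushes along a straight path and triggers a death event when it hits the player.
; StartTrain stores the BPMain reference, then a Timeline lerps the actor along world X with sweep and destroys it at the end.
; Two trigger boxes, each with its own DoOnce, pass an overlapping PlayerCharacter to BPMain's DeathFiveEvent.
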(event OnComponentBeginOverlap(Box)
  (params (OverlappedComponent :type Primitive%20Component%20Object%20Reference) (OtherActor :type Actor%20Object%20Reference) (OtherComp :type Primitive%20Component%20Object%20Reference) (OtherBodyIndex :type Integer) (bFromSweep :type Boolean) (SweepResult :type Hit%20Result%20Structure%20%28by%20ref%29))
  (bind _asplayer_character (Utilities|Casting|CastToPlayerCharacter OtherActor))
  (Utilities|FlowControl|DoOnce false
    (:Completed
      (Default|DeathFiveEvent (Variables|Default|GetBP%20Main) _asplayer_character))))

(event OnComponentBeginOverlap(Box1)
  (params (OverlappedComponent :type Primitive%20Component%20Object%20Reference) (OtherActor :type Actor%20Object%20Reference) (OtherComp :type Primitive%20Component%20Object%20Reference) (OtherBodyIndex :type Integer) (bFromSweep :type Boolean) (SweepResult :type Hit%20Result%20Structure%20%28by%20ref%29))
  (bind _asplayer_character (Utilities|Casting|CastToPlayerCharacter OtherActor))
  (Utilities|FlowControl|DoOnce false
    (:Completed
      (Default|DeathFiveEvent (Variables|Default|GetBP%20Main) _asplayer_character))))

(event Custom|StartTrain
  (params (BP_Main :type BP%20Main%20Anomaly%20Object%20Reference))
  (bind _returnvalue (Transformation|GetActorLocation))
  (Variables|Default|SetBP%20Main BP_Main)
  (Variables|Default|SetReturn%20Value%20Y (.y _returnvalue))
  (Variables|Default|SetReturn%20Value%20Z (.z _returnvalue))
  (Variables|Default|SetReturn%20Value%20X (.x _returnvalue))
  (Variables|Default|SetNewVar (+ (.x _returnvalue) 4e+03))
  (bind _newtrack_0 (Timeline|Timeline PlayFromStart)
    (:Update
      (Transformation|SetActorLocation (Math|Vector|MakeVector (Math|Float|Lerp (Variables|Default|GetReturn%20Value%20X) (Variables|Default|GetNewVar) _newtrack_0) (Variables|Default|GetReturn%20Value%20Y) (Variables|Default|GetReturn%20Value%20Z)) true false))
    (:Finished
      (Actor|DestroyActor))))

(fn ConstructionScript)