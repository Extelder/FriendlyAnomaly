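; Horror enemy pawn that, shortly after spawning, hunts the farthest living player and kills them on reaching them.
; BeginPlay scans all PlayerCharacters to pick that target, then chases it with AI MoveTo, retrying on failure.
; Success plays a loud attenuated sound and, with authority, calls Death on the player using the game instance's gameplay type.
; The pawn destroys itself after a successful catch or a fixed chase timeout.
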(event Custom|RunMulticastSound
  (Audio|PlaySoundatLocation "/Game/Blueprints/Sounds/67df2ab96dead2d.67df2ab96dead2d" (Transformation|GetActorLocation) "0, 0, 0" 3e+01 1.0 0.0 "/Game/Sound/SoundAttenuation/AnomalySpeaker.AnomalySpeaker" 0 0 0)
  (Networking|SwitchHasAuthority
    (:Authority
      (bind _asplayer_game_instance (Utilities|Casting|CastToPlayerGameInstance (Game|GetGameInstance)))
      (Default|Death (Variables|Default|GetPlayerCharacter) (Variables|/Game/Blueprints/Player/PlayerGameInstance.PlayerGameInstance_C|GetGameplayType _asplayer_game_instance) true))))

(event EventBeginPlay
  (Utilities|FlowControl|Delay 1.3)
  (bind _outactors (Actor|GetAllActorsOfClass "/Game/Blueprints/Player/Character/PlayerCharacter.PlayerCharacter_C"))
  (for _array_element _outactors
    (if (== (Variables|/Game/Blueprints/Player/Character/PlayerCharacter.PlayerCharacter_C|GetDeath1 _array_element) 0)
      (Utilities|IsValid (Variables|Default|GetPlayerCharacter)
        (:Is%20Valid
          (if (> (Transformation|GetDistanceTo _array_element) (Variables|Default|GetDistance))
            (Variables|Default|SetPlayerCharacter _array_element :!label _label)
            (Variables|Default|SetDistance (Transformation|GetDistanceTo _array_element))))
        (:Is%20Not%20Valid
          (goto _label)))))
  (AI|AIMoveTo self "0, 0, 0" (Variables|Default|GetPlayerCharacter) 5.0 false :!label _label_2
    (:then
      (Utilities|FlowControl|Delay 8.0))
    (:OnSuccess
      (CallFunction|RunMulticastSound))
    (:OnFail
      (Utilities|FlowControl|Sequence
        (:then_0
          (goto _label_2)))))
  (Actor|DestroyActor))

(fn ConstructionScript)

(fn RunMulticast)