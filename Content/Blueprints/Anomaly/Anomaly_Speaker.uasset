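; Speaker anomaly Blueprint: an interactable prop that plays either a normal or an anomalous sound.
; EnableAnomalybyIndex selects the sound (0 for normal, 1 for anomaly), and InteractableInteract spawns it attached to the static mesh.
; SetOverlayMaterial switches the overlay on SMWallLight01 between the outline and "AccupiedOutline" materials based on the Detect flag.
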(event EventSetOverlayMaterial
  (params (Detect :type Boolean))
  (bind _sm_wall_light_01 (Variables|Default|GetSM_wall_light_01))
  (if Detect
    (Rendering|Material|SetOverlayMaterial _sm_wall_light_01 (Variables|Default|GetOutlineMaterial) :!class /Script/Engine.MeshComponent)
    (else
      (Rendering|Material|SetOverlayMaterial _sm_wall_light_01 (Variables|Default|GetAccupiedOutline) :!class /Script/Engine.MeshComponent))))

(event EventEnableAnomalybyIndex
  (params (Index :type Integer))
  (switch int Index
    (:0
      (Variables|Default|SetSound "/Game/Sound/Speaker/Anomaly_SpeakerNorm.Anomaly_SpeakerNorm"))
    (:1
      (Variables|Default|SetSound "/Game/Sound/Speaker/Anomaly_Speaker.Anomaly_Speaker"))))

(event EventInteractableInteract
  (params (Player :type Player%20Character%20Object%20Reference))
  (Audio|SpawnSoundAttached (Variables|Default|GetSound) (Variables|Default|GetStaticMesh) "None" "0, 0, 0" "0, 0, 0" "KeepRelativeOffset" false 1.0 1.0 0.0 "/Game/Sound/SoundAttenuation/AnomalySpeaker.AnomalySpeaker" 0))

(fn ConstructionScript
  (|CallParentFunction))