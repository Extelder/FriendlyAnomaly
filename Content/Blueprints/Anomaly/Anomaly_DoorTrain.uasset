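; Anomaly variant of a train door whose two door panels can be shifted out of place.
; EnableAnomalybyIndex offsets the panels in opposite directions along world X, with the index choosing between two mirrored directions.
; SetOverlayMaterial switches both panels and the doorway mesh between the detect outline and the occupied outline based on the Detect flag.
; The construction script only runs the parent's logic.
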(event EventEnableAnomalybyIndex
  (params (Index :type Integer))
  (bind _sm_door_wall_04 (Variables|Default|GetSM_door_wall_04))
  (bind _sm_door_wall_03 (Variables|Default|GetSM_door_wall_03))
  (switch int Index
    (:0
      (Transformation|AddWorldOffset _sm_door_wall_04 "-66.000000,0.000000,0.000000" false false)
      (Transformation|AddWorldOffset _sm_door_wall_03 "66.000000,0.000000,0.000000" false false))
    (:1
      (Transformation|AddWorldOffset _sm_door_wall_04 "66.000000,0.000000,0.000000" false false)
      (Transformation|AddWorldOffset _sm_door_wall_03 "-66.000000,0.000000,0.000000" false false))))

(event EventSetOverlayMaterial
  (params (Detect :type Boolean))
  (bind _outlinematerial (Variables|Default|GetOutlineMaterial))
  (bind _accupiedoutline (Variables|Default|GetAccupiedOutline))
  (if Detect
    (Rendering|Material|SetOverlayMaterial (Variables|Default|GetSM_door_wall_03) _outlinematerial :!class /Script/Engine.MeshComponent)
    (Rendering|Material|SetOverlayMaterial (Variables|Default|GetSM_wall_doorway_02) _outlinematerial :!class /Script/Engine.MeshComponent)
    (Rendering|Material|SetOverlayMaterial (Variables|Default|GetSM_door_wall_04) _outlinematerial :!class /Script/Engine.MeshComponent)
    (else
      (Rendering|Material|SetOverlayMaterial (Variables|Default|GetSM_door_wall_03) _accupiedoutline :!class /Script/Engine.MeshComponent)
      (Rendering|Material|SetOverlayMaterial (Variables|Default|GetSM_wall_doorway_02) _accupiedoutline :!class /Script/Engine.MeshComponent)
      (Rendering|Material|SetOverlayMaterial (Variables|Default|GetSM_door_wall_04) _accupiedoutline :!class /Script/Engine.MeshComponent))))

(fn ConstructionScript
  (|CallParentFunction))