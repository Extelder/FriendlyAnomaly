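; Floor vent anomaly actor that switches its static mesh between a normal and an anomalous look.
; On BeginPlay it caches the mesh's first material as the default.
; EnableAnomalybyIndex selects the state: index 0 resets rotation and restores that material, while index 1 turns the mesh a quarter turn and applies the anomaly material.
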(event EventBeginPlay
  (Variables|Default|SetDefaultMaterial (Rendering|Material|GetMaterial (Variables|Default|GetStaticMesh) 0)))

(event EventEnableAnomalybyIndex
  (params (Index :type Integer))
  (switch int Index
    (:0
      (Transformation|SetRelativeRotation (Variables|Default|GetStaticMesh) "0, 0, 0" false false)
      (Rendering|Material|SetMaterial (Variables|Default|GetStaticMesh) 0 (Variables|Default|GetDefaultMaterial)))
    (:1
      (Transformation|SetRelativeRotation (Variables|Default|GetStaticMesh) "0.000000,90.000000,0.000000" false false)
      (Rendering|Material|SetMaterial (Variables|Default|GetStaticMesh) 0 (Variables|Default|GetAnomMaterial)))))

(fn ConstructionScript
  (|CallParentFunction))