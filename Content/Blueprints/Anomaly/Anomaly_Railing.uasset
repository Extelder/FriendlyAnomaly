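; Railing anomaly actor that switches two railing meshes between a normal state and two anomalous variants.
; EnableAnomalybyIndex selects default placement, a displaced AnomalyTransform placement, or default placement with the background material.
; SMRailing01 follows the main mesh's target transform at a fixed world X offset.
; SetOverlayMaterial swaps the outline overlay on SMRailing01 only, based on the Detect flag.
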(event EventSetOverlayMaterial
  (params (Detect :type Boolean))
  (bind _sm_railing01 (Variables|Default|GetSM_Railing01))
  (if Detect
    (Rendering|Material|SetOverlayMaterial _sm_railing01 (Variables|Default|GetOutlineMaterial) :!class /Script/Engine.MeshComponent)
    (else
      (Rendering|Material|SetOverlayMaterial _sm_railing01 (Variables|Default|GetAccupiedOutline) :!class /Script/Engine.MeshComponent))))

(event EventEnableAnomalybyIndex
  (params (Index :type Integer))
  (bind _sm_railing01 (Variables|Default|GetSM_Railing01))
  (bind _defaulttransform (Variables|Default|GetDefaultTransform))
  (bind _defaulttransform_2 (Variables|Default|GetDefaultTransform))
  (bind _anomalytransform (Variables|Default|GetAnomalyTransform))
  (bind _returnvalue (Transformation|GetWorldTransform _anomalytransform))
  (bind _returnvalue_2 (Transformation|GetWorldTransform _defaulttransform))
  (bind _returnvalue_3 (Transformation|GetWorldTransform _defaulttransform_2))
  (switch int Index
    (:0
      (Transformation|SetWorldTransform (Variables|Default|GetStaticMesh) (Transformation|GetWorldTransform (Variables|Default|GetDefaultTransform)) false false)
      (Transformation|SetWorldTransform _sm_railing01 (Math|Transform|MakeTransform (Math|Vector|MakeVector (+ (.x (.location _returnvalue_2)) 491.0) (.y (.location _returnvalue_2)) (.z (.location _returnvalue_2))) (.rotation _returnvalue_2) (.scale _returnvalue_2)) false false)
      (Rendering|Material|SetMaterial (Variables|Default|GetStaticMesh) 0 "/Game/Subway/Materials/Platform/Railing/MI_Railing.MI_Railing")
      (Rendering|Material|SetMaterial (Variables|Default|GetSM_Railing01) 0 "/Game/Subway/Materials/Platform/Railing/MI_Railing.MI_Railing"))
    (:1
      (Transformation|SetWorldTransform (Variables|Default|GetStaticMesh) (Transformation|GetWorldTransform (Variables|Default|GetAnomalyTransform)) false false)
      (Transformation|SetWorldTransform _sm_railing01 (Math|Transform|MakeTransform (Math|Vector|MakeVector (+ (.x (.location _returnvalue)) 491.0) (.y (.location _returnvalue)) (.z (.location _returnvalue))) (.rotation _returnvalue) (.scale _returnvalue)) false false)
      (Rendering|Material|SetMaterial (Variables|Default|GetStaticMesh) 0 "/Game/Subway/Materials/Platform/Railing/MI_Railing.MI_Railing")
      (Rendering|Material|SetMaterial (Variables|Default|GetSM_Railing01) 0 "/Game/Subway/Materials/Platform/Railing/MI_Railing.MI_Railing"))
    (:2
      (Transformation|SetWorldTransform (Variables|Default|GetStaticMesh) (Transformation|GetWorldTransform (Variables|Default|GetDefaultTransform)) false false)
      (Transformation|SetWorldTransform (Variables|Default|GetSM_Railing01) (Math|Transform|MakeTransform (Math|Vector|MakeVector (+ (.x (.location _returnvalue_3)) 491.0) (.y (.location _returnvalue_3)) (.z (.location _returnvalue_3))) (.rotation _returnvalue_3) (.scale _returnvalue_3)) false false)
      (Rendering|Material|SetMaterial (Variables|Default|GetStaticMesh) 0 "/Engine/EngineMeshes/BackgroundMaterial.BackgroundMaterial")
      (Rendering|Material|SetMaterial (Variables|Default|GetSM_Railing01) 0 "/Engine/EngineMeshes/BackgroundMaterial.BackgroundMaterial"))))

(fn ConstructionScript
  (|CallParentFunction))