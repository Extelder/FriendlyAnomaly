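; Anomaly_Trashcan is an anomaly actor that switches a trashcan mesh between its normal and anomalous placement.
; EnableAnomalybyIndex snaps StaticMesh to the world transform of the Default component for index 0 or the Anomaly component for index 1.
; The two components act as transform markers, and the construction script only calls its parent.
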(event EventEnableAnomalybyIndex
  (params (Index :type Integer))
  (switch int Index
    (:0
      (Transformation|SetWorldTransform (Variables|Default|GetStaticMesh) (Transformation|GetWorldTransform (Variables|Default|GetDefault)) false false))
    (:1
      (Transformation|SetWorldTransform (Variables|Default|GetStaticMesh) (Transformation|GetWorldTransform (Variables|Default|GetAnomaly)) false false))))

(fn ConstructionScript
  (|CallParentFunction))