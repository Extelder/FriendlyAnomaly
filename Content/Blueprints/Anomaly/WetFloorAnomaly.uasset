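; Wet floor anomaly actor that switches its static mesh between a normal state and an anomalous one, selected by index.
; The Default and Stand components serve as placement markers whose relative transforms are copied onto the mesh.
; EnableAnomalybyIndex applies either the default placement with the original material cached at BeginPlay, or the Stand placement with an anomaly material.
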(event EventBeginPlay
  (Variables|Default|SetDefaultMaterial (Rendering|Material|GetMaterial (Variables|Default|GetStaticMesh) 0)))

(event EventEnableAnomalybyIndex
  (params (Index :type Integer))
  (switch int Index
    (:0
      (Transformation|SetRelativeTransform (Variables|Default|GetStaticMesh) (Transformation|GetRelativeTransform (Variables|Default|GetDefault)) false false)
      (Rendering|Material|SetMaterial (Variables|Default|GetStaticMesh) 0 (Variables|Default|GetDefaultMaterial)))
    (:1
      (Transformation|SetRelativeTransform (Variables|Default|GetStaticMesh) (Transformation|GetRelativeTransform (Variables|Default|GetStand)) false false)
      (Rendering|Material|SetMaterial (Variables|Default|GetStaticMesh) 0 (Variables|Default|GetAnomMaterial)))))

(fn ConstructionScript
  (|CallParentFunction))