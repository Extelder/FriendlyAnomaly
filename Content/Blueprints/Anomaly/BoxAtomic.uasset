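; BoxAtomic is an anomaly actor that switches a box prop between two static mesh variants.
; EnableAnomalybyIndex shows StaticMesh for index 0 or StaticMesh1 for index 1 and hides the other.
; SetOverlayMaterial applies one of two outline overlays to StaticMesh1 only, chosen by the Detect flag.
; The construction script only calls the parent's version.
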(event EventSetOverlayMaterial
  (params (Detect :type Boolean))
  (bind _staticmesh1 (Variables|Default|GetStaticMesh1))
  (if Detect
    (Rendering|Material|SetOverlayMaterial _staticmesh1 (Variables|Default|GetOutlineMaterial) :!class /Script/Engine.MeshComponent)
    (else
      (Rendering|Material|SetOverlayMaterial _staticmesh1 (Variables|Default|GetAccupiedOutline) :!class /Script/Engine.MeshComponent))))

(event EventEnableAnomalybyIndex
  (params (Index :type Integer))
  (switch int Index
    (:0
      (Rendering|SetVisibility (Variables|Default|GetStaticMesh) true false)
      (Rendering|SetVisibility (Variables|Default|GetStaticMesh1) false false))
    (:1
      (Rendering|SetVisibility (Variables|Default|GetStaticMesh) false false)
      (Rendering|SetVisibility (Variables|Default|GetStaticMesh1) true false))))

(fn ConstructionScript
  (|CallParentFunction))