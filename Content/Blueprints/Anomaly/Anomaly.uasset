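; Base anomaly actor for a hider-versus-seeker game: hiders cycle its anomaly state, and seekers mark it as a guess.
; A hider claims it while under a three-anomaly limit, and changes route through the owner's server call, with multicast events applying the index.
; Seeker toggles report right or wrong picks based on whether the index is non-zero.
; Overlay outlines show detection and selection; state-switching and extra overlay functions are empty stubs.
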(event Custom|EnableAnomalyMulticast
  (params (Index :type Integer))
  (CallFunction|EnableAnomalybyIndex Index))

(event Custom|EnableAnomalyOnServer
  (params (Index :type Integer))
  (CallFunction|EnableAnomalyMulticast Index))

(event Custom|RandomOnServer
  (CallFunction|RandomMulticast (Math|Random|RandomIntegerinRange 0 (Variables|Default|GetIndexCapacity))))

(event Custom|OnServer
  ;[1 1 1] Debug
)

(event Custom|RandomMulticast
  (params (Index :type Integer))
  (CallFunction|EnableAnomalybyIndex Index))

(event Custom|ChangeAnomalyByHider
  (params (Owner :type Player%20Character%20Object%20Reference))
  (bind _self self)
  (if (== (Variables|Default|GetCurrentIndex) (Variables|Default|GetIndexCapacity))
    (bind _output_get (Variables|Default|SetCurrentIndex 0))
    (Default|ChangeAnomalyonServer Owner _output_get (Variables|Default|GetCurrentHider) _self)
    (else
      (bind _output_get_2 (Variables|Default|SetCurrentIndex (+ (Variables|Default|GetCurrentIndex) 1)))
      (Default|ChangeAnomalyonServer Owner _output_get_2 (Variables|Default|GetCurrentHider) _self)))
  (if (!= (Variables|Default|GetCurrentIndex) 0)
    (if (not (> (Variables|Default|GetCurrentIndex) 1))
      (Utilities|IsValid (Variables|Default|GetCurrentHider)
        (:Is%20Valid
          _)
        (:Is%20Not%20Valid
          _))
      (Variables|Default|SetAccupiedOutline "/Game/Materials/Outline1.Outline1"))
    (else
      (Utilities|IsValid (Variables|Default|GetCurrentHider)
        (:Is%20Valid
          (Variables|Default|SetCurrentHider 0))
        (:Is%20Not%20Valid
          _))
      (Variables|Default|SetAccupiedOutline 0))))

(event Custom|SetAnomalyBySeeker
  (params (Seeker :type Seeker%20Object%20Reference))
  (bind _currentindex (Variables|Default|GetCurrentIndex))
  (bind _returnvalue (!= _currentindex 0))
  (Variables|Default|SetNowChoice (not (Variables|Default|GetNowChoice)))
  (Utilities|IsValid Seeker
    (:Is%20Valid
      (if (Variables|Default|GetNowChoice)
        (if _returnvalue
          (Default|AddonServer Seeker true true)
          (else
            (Default|AddonServer Seeker true false)))
        (Variables|Default|SetAccupiedOutline "/Game/Materials/Outline2.Outline2")
        (else
          (if _returnvalue
            (Default|AddonServer Seeker false true)
            (else
              (Default|AddonServer Seeker false false)))
          (Variables|Default|SetAccupiedOutline 0))))))

(event Custom|SeekerLostByMainAnomalia
  (Variables|Default|SetAccupiedOutline 0)
  (Rendering|Material|SetOverlayMaterial (Variables|Default|GetStaticMesh) (Variables|Default|GetAccupiedOutline) :!class /Script/Engine.MeshComponent)
  (CallFunction|SetOverlayMaterial false)
  (Variables|Default|SetNowChoice false))

(event Custom|ChangeAnomalyOnMulticast
  (params (Index :type Integer) (Hider :type Hider%20Object%20Reference))
  (bind _currentanomalies (Variables|/Game/Blueprints/Player/Hider/Hider.Hider_C|GetCurrentAnomalies Hider))
  (CallFunction|EnableAnomalybyIndex Index)
  (Variables|Default|SetCurrentIndex Index)
  (if (!= Index 0)
    (if (not (> Index 1))
      (Math|Integer|IncrementInt _currentanomalies))
    (else
      (Math|Integer|DecrementInt _currentanomalies))))

(event EventDetect
  (Rendering|Material|SetOverlayMaterial (Variables|Default|GetStaticMesh) (Variables|Default|GetOutlineMaterial) :!class /Script/Engine.MeshComponent)
  (CallFunction|SetOverlayMaterial true))

(event EventLost
  (Rendering|Material|SetOverlayMaterial (Variables|Default|GetStaticMesh) (Variables|Default|GetAccupiedOutline) :!class /Script/Engine.MeshComponent)
  (CallFunction|SetOverlayMaterial false))

(event EventInteract
  (params (Hider :type Hider%20Object%20Reference) (Owner :type Player%20Character%20Object%20Reference))
  (Audio|PlaySound2D "/Game/Sound/Interact/InteractRandom.InteractRandom" 1.0 1.0 0.0 0 0)
  (Utilities|IsValid (Variables|Default|GetCurrentHider)
    (:Is%20Valid
      (if (== Hider (Variables|Default|GetCurrentHider))
        (Variables|Default|SetCurrentHider Hider :!label _label)
        (CallFunction|ChangeAnomalybyHider Owner)))
    (:Is%20Not%20Valid
      (if (< (Variables|/Game/Blueprints/Player/Hider/Hider.Hider_C|GetCurrentAnomalies Hider) 3)
        (goto _label)))))

(event EventEnableAnomaly
  (params (Index :type Integer))
  (CallFunction|EnableAnomalyonServer Index))

(event EventEnableRandomAnomaly)

(event EventSeekerDetect
  (Rendering|Material|SetOverlayMaterial (Variables|Default|GetStaticMesh) (Variables|Default|GetOutlineMaterial) :!class /Script/Engine.MeshComponent)
  (CallFunction|SetOverlayMaterial true))

(event EventSeekerLost
  (Rendering|Material|SetOverlayMaterial (Variables|Default|GetStaticMesh) (Variables|Default|GetAccupiedOutline) :!class /Script/Engine.MeshComponent)
  (CallFunction|SetOverlayMaterial false))

(event EventSeekerInteract
  (params (Seeker :type Seeker%20Object%20Reference))
  (CallFunction|SetAnomalybySeeker Seeker))

(event EventTick
  (params (DeltaSeconds :type Float%20%28single-precision%29))
  ;[1 1 1] Debug
)

(fn ConstructionScript)

(fn EnableAnomalybyIndex
  (params (Index :type Integer)))

(fn SetOverlayMaterial
  (params (Detect :type Boolean)))