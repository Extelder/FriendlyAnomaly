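; Bench anomaly actor that switches between a normal bench and an anomalous variant.
; EnableAnomalybyIndex swaps the main mesh between default and anomaly versions and hides or shows a secondary mesh with its children.
; SetOverlayMaterial applies one of two outline overlay materials to all four bench meshes, depending on the Detect flag.
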(event EventSetOverlayMaterial
  (params (Detect :type Boolean))
  (bind _outlinematerial (Variables|Default|GetOutlineMaterial))
  (bind _accupiedoutline (Variables|Default|GetAccupiedOutline))
  (if Detect
    (Rendering|Material|SetOverlayMaterial (Variables|Default|GetStaticMesh) _outlinematerial :!class /Script/Engine.MeshComponent)
    (Rendering|Material|SetOverlayMaterial (Variables|Default|GetStaticMesh2) _outlinematerial :!class /Script/Engine.MeshComponent)
    (Rendering|Material|SetOverlayMaterial (Variables|Default|GetStaticMesh3) _outlinematerial :!class /Script/Engine.MeshComponent)
    (Rendering|Material|SetOverlayMaterial (Variables|Default|GetStaticMesh1) _outlinematerial :!class /Script/Engine.MeshComponent)
    (else
      (Rendering|Material|SetOverlayMaterial (Variables|Default|GetStaticMesh) _accupiedoutline :!class /Script/Engine.MeshComponent)
      (Rendering|Material|SetOverlayMaterial (Variables|Default|GetStaticMesh2) _accupiedoutline :!class /Script/Engine.MeshComponent)
      (Rendering|Material|SetOverlayMaterial (Variables|Default|GetStaticMesh3) _accupiedoutline :!class /Script/Engine.MeshComponent)
      (Rendering|Material|SetOverlayMaterial (Variables|Default|GetStaticMesh1) _accupiedoutline :!class /Script/Engine.MeshComponent))))

(event EventEnableAnomalybyIndex
  (params (Index :type Integer))
  (bind _staticmesh2 (Variables|Default|GetStaticMesh2))
  (switch int Index
    (:0
      (Components|StaticMesh|SetStaticMesh (Variables|Default|GetStaticMesh) (Variables|Default|GetDefaultBench))
      (Rendering|SetVisibility _staticmesh2 false true))
    (:1
      (Components|StaticMesh|SetStaticMesh (Variables|Default|GetStaticMesh) (Variables|Default|GetAnomalyBench))
      (Rendering|SetVisibility _staticmesh2 true true))))

(fn ConstructionScript
  (|CallParentFunction))