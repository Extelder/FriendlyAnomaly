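; Anomaly actor that shows a man and woman mesh pair in a normal, anomalous or trap variant.
; An index event restores the default layout, swaps the meshes with an anomaly material, or keeps the layout and puts a trap material on StaticMesh1.
; The default material is cached from StaticMesh on BeginPlay.
; A detection flag switches the overlay outline, which applies only to StaticMesh1.
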(event EventBeginPlay
  (Variables|Default|SetDefaultMaterial (Rendering|Material|GetMaterial (Variables|Default|GetStaticMesh) 0)))

(event EventSetOverlayMaterial
  (params (Detect :type Boolean))
  (if Detect
    (Rendering|Material|SetOverlayMaterial (Variables|Default|GetStaticMesh1) (Variables|Default|GetOutlineMaterial) :!class /Script/Engine.MeshComponent)
    (else
      (Rendering|Material|SetOverlayMaterial (Variables|Default|GetStaticMesh1) (Variables|Default|GetAccupiedOutline) :!class /Script/Engine.MeshComponent))))

(event EventEnableAnomalybyIndex
  (params (Index :type Integer))
  (bind _staticmesh (Variables|Default|GetStaticMesh))
  (bind _staticmesh1 (Variables|Default|GetStaticMesh1))
  (bind _staticmesh1_2 (Variables|Default|GetStaticMesh1))
  (switch int Index
    (:0
      (Components|StaticMesh|SetStaticMesh _staticmesh1 (Variables|Default|GetWoman))
      (Components|StaticMesh|SetStaticMesh (Variables|Default|GetStaticMesh) (Variables|Default|GetMan))
      (Rendering|Material|SetMaterial _staticmesh1 0 (Variables|Default|GetDefaultMaterial)))
    (:1
      (Components|StaticMesh|SetStaticMesh _staticmesh (Variables|Default|GetWoman))
      (Components|StaticMesh|SetStaticMesh (Variables|Default|GetStaticMesh1) (Variables|Default|GetMan))
      (Rendering|Material|SetMaterial _staticmesh 0 (Variables|Default|GetAnomMaterial)))
    (:2
      (Components|StaticMesh|SetStaticMesh _staticmesh1_2 (Variables|Default|GetWoman))
      (Components|StaticMesh|SetStaticMesh (Variables|Default|GetStaticMesh) (Variables|Default|GetMan))
      (Rendering|Material|SetMaterial _staticmesh1_2 0 (Variables|Default|GetDefaultMaterial))
      (Rendering|Material|SetMaterial (Variables|Default|GetStaticMesh1) 0 "/Game/Subway/Materials/Platform/Signs/Trap.Trap"))))

(fn ConstructionScript
  (|CallParentFunction))