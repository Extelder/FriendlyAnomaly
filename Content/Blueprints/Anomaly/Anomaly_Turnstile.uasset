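; Turnstile anomaly actor that switches between visual variants by index.
; EnableAnomalybyIndex sets the default look, mirrors the three static meshes through negative Y scale, or mirrors them and also reveals the three Skuku components.
; SetOverlayMaterial swaps the overlay on two of the meshes between the outline and occupied-outline materials according to the Detect flag.
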(event EventSetOverlayMaterial
  (params (Detect :type Boolean))
  (if Detect
    (Rendering|Material|SetOverlayMaterial (Variables|Default|GetStaticMesh2) (Variables|Default|GetOutlineMaterial) :!class /Script/Engine.MeshComponent)
    (Rendering|Material|SetOverlayMaterial (Variables|Default|GetStaticMesh1) (Variables|Default|GetOutlineMaterial) :!class /Script/Engine.MeshComponent)
    (else
      (Rendering|Material|SetOverlayMaterial (Variables|Default|GetStaticMesh2) (Variables|Default|GetAccupiedOutline) :!class /Script/Engine.MeshComponent)
      (Rendering|Material|SetOverlayMaterial (Variables|Default|GetStaticMesh1) (Variables|Default|GetAccupiedOutline) :!class /Script/Engine.MeshComponent))))

(event EventEnableAnomalybyIndex
  (params (Index :type Integer))
  (switch int Index
    (:0
      (Transformation|SetRelativeScale3D (Variables|Default|GetStaticMesh) "1.000000,1.000000,1.000000")
      (Transformation|SetRelativeScale3D (Variables|Default|GetStaticMesh1) "1.000000,1.000000,1.000000")
      (Transformation|SetRelativeScale3D (Variables|Default|GetStaticMesh2) "1.000000,1.000000,1.000000")
      (Rendering|SetVisibility (Variables|Default|Getskuku) false false :!label _label))
    (:1
      (Transformation|SetRelativeScale3D (Variables|Default|GetStaticMesh) "1.000000,-1.000000,1.000000")
      (Transformation|SetRelativeScale3D (Variables|Default|GetStaticMesh1) "1.000000,-1.000000,1.000000")
      (Transformation|SetRelativeScale3D (Variables|Default|GetStaticMesh2) "1.000000,-1.000000,1.000000")
      (goto _label))
    (:2
      (Transformation|SetRelativeScale3D (Variables|Default|GetStaticMesh) "1.000000,-1.000000,1.000000")
      (Transformation|SetRelativeScale3D (Variables|Default|GetStaticMesh1) "1.000000,-1.000000,1.000000")
      (Transformation|SetRelativeScale3D (Variables|Default|GetStaticMesh2) "1.000000,-1.000000,1.000000")
      (Rendering|SetVisibility (Variables|Default|Getskuku) true false))))

(fn ConstructionScript
  (|CallParentFunction))