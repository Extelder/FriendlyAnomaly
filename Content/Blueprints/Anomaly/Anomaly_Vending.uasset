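; Vending machine anomaly actor that switches its mesh between a normal look and an anomalous one.
; BeginPlay applies the default material to the first slot of the static mesh.
; EnableAnomalybyIndex then selects the default or anomaly material for that slot from the index it receives.
; The construction script only calls the parent version.
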(event EventBeginPlay
  (Rendering|Material|SetMaterial (Variables|Default|GetStaticMesh) 0 (Variables|Default|GetDefaultMaterial)))

(event EventEnableAnomalybyIndex
  (params (Index :type Integer))
  (switch int Index
    (:0
      (Rendering|Material|SetMaterial (Variables|Default|GetStaticMesh) 0 (Variables|Default|GetDefaultMaterial)))
    (:1
      (Rendering|Material|SetMaterial (Variables|Default|GetStaticMesh) 0 (Variables|Default|GetAnomalyMaterial)))))

(fn ConstructionScript
  (|CallParentFunction))