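; Camera anomaly actor that shows one of two camera component variants and outlines the current one.
; EnableAnomalybyIndex makes either Camera or Camera1 visible and hides the other, based on the given index.
; SetOverlayMaterial uses CurrentIndex to pick the component, then applies OutlineMaterial when detected or AccupiedOutline otherwise.
; The construction script only calls its parent.
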(event EventEnableAnomalybyIndex
  (params (Index :type Integer))
  (switch int Index
    (:0
      (Rendering|SetVisibility (Variables|Default|GetCamera) true false)
      (Rendering|SetVisibility (Variables|Default|GetCamera1) false false))
    (:1
      (Rendering|SetVisibility (Variables|Default|GetCamera) false false)
      (Rendering|SetVisibility (Variables|Default|GetCamera1) true false))))

(event EventSetOverlayMaterial
  (params (Detect :type Boolean))
  (bind _camera1 (Variables|Default|GetCamera1))
  (bind _currentindex (Variables|Default|GetCurrentIndex))
  (bind _returnvalue (== _currentindex 0))
  (if Detect
    (if _returnvalue
      (Rendering|Material|SetOverlayMaterial (Variables|Default|GetCamera) (Variables|Default|GetOutlineMaterial) :!class /Script/Engine.MeshComponent)
      (else
        (Rendering|Material|SetOverlayMaterial _camera1 (Variables|Default|GetOutlineMaterial) :!class /Script/Engine.MeshComponent)))
    (elif _returnvalue
      (Rendering|Material|SetOverlayMaterial (Variables|Default|GetCamera) (Variables|Default|GetAccupiedOutline) :!class /Script/Engine.MeshComponent)
      (else
        (Rendering|Material|SetOverlayMaterial _camera1 (Variables|Default|GetAccupiedOutline) :!class /Script/Engine.MeshComponent)))))

(fn ConstructionScript
  (|CallParentFunction))