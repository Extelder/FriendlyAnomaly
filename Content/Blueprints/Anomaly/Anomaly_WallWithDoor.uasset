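; Anomaly actor for a wall with a door, which changes the door's appearance by anomaly index.
; EnableAnomalybyIndex switches on the index to set visibility of two door parts: index 0 shows both, while index 1 hides DoorPart2 and keeps DoorPart1 visible.
; The construction script only defers to the parent class.
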(event EventEnableAnomalybyIndex
  (params (Index :type Integer))
  (switch int Index
    (:0
      (Rendering|SetVisibility (Variables|Default|GetDoorPart2) true false)
      (Rendering|SetVisibility (Variables|Default|GetDoorPart1) true false))
    (:1
      (Rendering|SetVisibility (Variables|Default|GetDoorPart2) false false)
      (Rendering|SetVisibility (Variables|Default|GetDoorPart1) true false))))

(fn ConstructionScript
  (|CallParentFunction))