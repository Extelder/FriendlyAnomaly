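; Anomaly actor for an ATM prop that changes its appearance according to an anomaly index.
; EnableAnomalybyIndex swaps the static mesh's first material between the base, anomaly and casino variants.
; Disconnected nodes that would move the mesh between Default and Anomaly transforms remain unused, and the construction script only calls its parent.
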(event EventEnableAnomalybyIndex
  (params (Index :type Integer))
  (bind _staticmesh (Variables|Default|GetStaticMesh))
  (switch int Index
    (:0
      (Rendering|Material|SetMaterial _staticmesh 0 "/Game/Meshes/ATM/Base.Base"))
    (:1
      (Rendering|Material|SetMaterial _staticmesh 0 "/Game/Meshes/ATM/BaseAnomaly.BaseAnomaly"))
    (:2
      (Rendering|Material|SetMaterial _staticmesh 0 "/Game/Meshes/ATM/Casino.Casino"))))

(fn ConstructionScript
  (|CallParentFunction))