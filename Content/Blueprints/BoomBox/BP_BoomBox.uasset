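; BP_BoomBox is a boombox actor that plays songs from a NewSound list through its Audio component.
; SetSoundByOne sets the sound at a given index and plays it from the start.
; SetSound advances IDCurrentSong, wrapping to the first track after the last, and passes it to SetSoundByOne.
; Picking a track directly does not update IDCurrentSong, and the construction script is empty.
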(event Custom|SetSound
  ;[1 1 1] Set Music
  (if (== (Variables|Default|GetIDCurrentSong) (- (Utilities|Array|Length (Variables|Default|GetNew%20Sound)) 1))
    (Variables|Default|SetIDCurrentSong 0)
    (else
      (Math|Integer|IncrementInt (Variables|Default|GetIDCurrentSong)
        (:%20%20
          _))))
  (CallFunction|SetSoundbyOne (Variables|Default|GetIDCurrentSong)))

(event Custom|SetSoundByOne
  (params (Song :type Integer))
  (bind _audio (Variables|Default|GetAudio))
  ;[1 1 1] Set Music
  (Audio|Components|Audio|SetSound _audio (Utilities|Array|Get(acopy) (Variables|Default|GetNew%20Sound) Song))
  (Audio|Components|Audio|Play _audio 0.0))

(fn ConstructionScript)