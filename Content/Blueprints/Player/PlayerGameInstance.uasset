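; Player game instance that manages multiplayer sessions via Advanced Sessions: hosting, searching, joining, invites and network error messages.
; Each session action first destroys any existing session; public hosting tags a random code and opens a listen-server lobby.
; StartGame requires two players, then server-travels to Subway, or SubwayHall during a late-October to mid-November window.
; It also refreshes on login/logout, saves a tutorial flag and launches survey and Steam links on shutdown.
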(event Custom|StartGame
  ;[1 1 1] StartGame
  (Utilities|FlowControl|DoN 1 :!label _label
    (:Exit
      (if (< (Utilities|Array|Length (Variables|/Script/Engine.GameStateBase|GetPlayerArray (Game|GetGameState))) 2)
        (Development|PrintString "Invite at least one person" true true "(R=1.000000,G=0.000000,B=0.907705,A=1.000000)" 5.0)
        (bind _foundwidgets (Widget|GetAllWidgetsOfClass "/Game/Lobby/Loading/WBP_Loading.WBP_Loading_C" true))
        (Widget|RemovefromParent (Utilities|Array|Get(acopy) _foundwidgets))
        (goto _label Reset)
        (else
          (Variables|Default|SetAllUSers (Utilities|Array|Length (Variables|/Script/Engine.GameStateBase|GetPlayerArray (Game|GetGameState))))
          (bind _hallowen_ (CallFunction|TimeGet))
          (if _hallowen_
            (bind _returnvalue (Class|AdvancedSessionsLibrary|ServerTravel "/Game/Maps/SubwayHall?listen" true false))
            (if (not _returnvalue)
              (Development|PrintString "Error: FailServerTravel" true true "(R=1.000000,G=0.000000,B=0.062383,A=1.000000)" 15.0 :!label _label_2))
            (else
              (bind _returnvalue_2 (Class|AdvancedSessionsLibrary|ServerTravel "/Game/Maps/Subway?listen" true false))
              (if (not _returnvalue_2)
                (goto _label_2)))))))))

(event Custom|SetPlayerGameplayType
  (params (Player%20Type :type PlayerType%20Enum :default "NewEnumerator0"))
  ;[1 0 0.01764] Joining
  (Variables|Default|SetGameplayType Player%20Type))

(event Custom|NewPlayerLogin
  (params (PlayerController :type Player%20Controller%20Object%20Reference))
  ;[1 1 1] PostLogin/OnLogout
  (Default|CallPlayerLogin))

(event Custom|Host
  (params (Random? :type Boolean) (Invite%20Only? :type Boolean) (Friends%20Only? :type Boolean) (Public%20Lobby? :type Boolean) (Lan :type Boolean))
  (bind _self self)
  ;[1 0 0.01764] Hosting
  (|DestroySession (Game|GetPlayerController 0)
    (:OnSuccess
      _)
    (:OnFailure
      _))
  (if Public%20Lobby?
    (Utilities|FlowControl|Delay 1.0)
    (bind _code (CallFunction|GetRandomCode))
    (|AdvancedSession (Utilities|Array|MakeArray (Class|AdvancedSessionsLibrary|MakeLiteralSessionPropertyString "CODE" _code)) (Game|GetPlayerController 0) 5 5 false true false true true true false false false true false true
      (:OnSuccess
        (if Random?
          (Variables|PlayerGameInstance_C|SetGameplayType _self "NewEnumerator0")
          (else
            (Variables|Default|SetGameComplexetty "NewEnumerator3")
            (Variables|PlayerGameInstance_C|SetGameplayType _self "NewEnumerator1")))
        (Game|OpenLevel(byObjectReference) "/Game/Lobby/MenuSubwayStart.MenuSubwayStart" true "listen"))
      (:OnFailure
        (Development|PrintString "Failure")))))

(event Custom|Join
  (params (SearchResult :type Blueprint%20Session%20Result%20Structure%20%28by%20ref%29))
  (|DestroySession (Game|GetPlayerController 0)
    (:OnSuccess
      _)
    (:OnFailure
      _))
  ;[1 0 0.01764] Joining
  (|JoinSession (Game|GetPlayerController 0) SearchResult
    (:OnFailure
      (Development|PrintString "FailSessions" true true "(R=1.000000,G=0.008842,B=0.000000,A=1.000000)" 1e+01)
      (|DestroySession (Game|GetPlayerController 0)))))

(event Custom|NewPlayerOnLogout
  (params (NetID :type Unique%20Net%20Id%20Repl%20Structure))
  ;[1 1 1] PostLogin/OnLogout
  (Default|CallPlayerLogin))

(event Custom|GetServers
  (params (WidgetRef :type Server%20List%20Object%20Reference))
  (bind _returnvalue (Game|GetPlayerController 0))
  ;[1 0 0.01764] Joining
  (|DestroySession _returnvalue
    (:OnSuccess
      _)
    (:OnFailure
      _))
  (bind _results (|FindSessionsAdvanced _returnvalue 100 false "AllServers" 0 false false false true)
    (:OnSuccess
      (Default|ClickJoin WidgetRef _results true))
    (:OnFailure
      (Utilities|IsValid WidgetRef
        (:Is%20Valid
          (Default|ClickJoin WidgetRef 0 false))))))

(event Custom|Teach
  (bind _returnvalue (SaveGame|CreateSaveGameObject "/Game/Blueprints/Player/BP_SaveGame.BP_SaveGame_C"))
  (Variables|/Game/Blueprints/Player/BP_SaveGame.BP_SaveGame_C|SetTeach? _returnvalue true)
  (SaveGame|SaveGametoSlot _returnvalue "Anomaly"))

(event EventOnSessionInviteAccepted
  (params (LocalPlayerNum :type Integer) (PersonInvited :type BP%20Unique%20Net%20Id%20Structure) (SessionToJoin :type Blueprint%20Session%20Result%20Structure%20%28by%20ref%29))
  (bind _returnvalue (Game|GetPlayerController 0))
  ;[1 0.1116 0.1813] Accept Invite
  (|DestroySession _returnvalue
    (:OnSuccess
      _)
    (:OnFailure
      _))
  (Variables|Default|SetTypeConnection "NewEnumerator1")
  (Utilities|FlowControl|Delay 0.2)
  (|JoinSession _returnvalue SessionToJoin
    (:OnSuccess
      (Development|PrintString "Invite Accepted. Joining..."))
    (:OnFailure
      (Development|PrintString "Session Join Failure!"))))

(event EventHandleNetworkError
  (params (FailureType :type ENetworkFailure%20Enum :default "NetDriverAlreadyExists") (bIsServer :type Boolean))
  ;[1 1 1] ServerError
  (Development|PrintString (Utilities|String|EnumtoString FailureType) true true "(R=1.000000,G=0.121763,B=0.000000,A=1.000000)" 7.0))

(event EventHandleTravelError
  (params (FailureType :type ETravelFailure%20Enum :default "NoLevel"))
  ;[1 1 1] ServerError
  (Development|PrintString (Utilities|String|EnumtoString FailureType) true true "(R=1.000000,G=0.097827,B=0.000000,A=1.000000)" 7.0))

(event EventOnSessionInviteReceived
  (params (LocalPlayerNum :type Integer) (PersonInviting :type BP%20Unique%20Net%20Id%20Structure) (AppId :type String) (SessionToJoin :type Blueprint%20Session%20Result%20Structure%20%28by%20ref%29))
  (bind _returnvalue (Game|GetPlayerController 0))
  ;[1 0.1116 0.1813] Accept Invite
  (|DestroySession _returnvalue
    (:OnSuccess
      _)
    (:OnFailure
      _))
  (Variables|Default|SetTypeConnection "NewEnumerator1")
  (Utilities|FlowControl|Delay 0.2)
  (|JoinSession _returnvalue SessionToJoin
    (:OnSuccess
      (Development|PrintString "Invite Accepted. Joining..."))
    (:OnFailure
      (Development|PrintString "Session Join Failure! Two"))))

(event EventShutdown
  ;[1 1 1] KARITEI FILES
  ;;[1 1 1] TOP SECRET
  ;;;[1 1 1] DO NOT USE
  ;;;;[1 1 1] hgy8ughduyi
  ;;;;;[1 1 1] lPSICongro
  ;;;;;;[1 1 1] 8geoalpha
  ;;;;;;;[1 1 1] THIS MUSTN`T BE LIVE
  ;;;;;;;;[1 1 1] SHIT
  ;;;;;;;;;[1 1 1] DO NOT GO NEAR PLEASE!!!
  ;;;;;;;;;;[1 1 1] FUCK NO...
  ;;;;;;;;;;;[1 1 1] WARNING
  ;;;;;;;;;;;;[1 1 1] !!DO NOT ENABLE!! GAME DEATH WARNING!!
  (Utilities|Platform|LaunchURL "https://forms.gle/6fw1ZUzhyRKhoVcz7")
  (Utilities|Platform|LaunchURL "steam://store/3981970"))

(fn CasttoServer)

(fn MultiCast)

(fn TimeGet
  (bind _returnvalue (Math|DateTime|Now))
  (bind _returnvalue_2 (Class|KismetMathLibrary|GetDate _returnvalue))
  (bind _returnvalue_3 (Class|KismetMathLibrary|GetMonth _returnvalue_2))
  (bind _returnvalue_4 (Class|KismetMathLibrary|GetDay _returnvalue_2))
  (if (or (and (== _returnvalue_3 11) (<= _returnvalue_4 12)) (and (== _returnvalue_3 10) (>= _returnvalue_4 20)))
    (return true)
    (else
      (return false))))

(fn GetRandomCode
  (for _index (range 1 6)
    (LocalVariables|SetString (Utilities|String|Append (LocalVariables|GetString) (Class|KismetStringLibrary|Mid (LocalVariables|GetAlf) (Math|Random|RandomIntegerinRange 1 35) 1))))
  (return (LocalVariables|GetString)))