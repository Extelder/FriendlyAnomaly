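; MainPlayerGameState is a game state that runs a replicated match countdown and shows it on the local player's TimerDisplay.
; StartTimer starts a one-second looping timer that decrements TimeCounter and refreshes the display through a cached PlayerCharacter.
; Every ten ticks the authority copies the count into TimeChecker, whose OnRep corrects drifted copies and restarts their timer, avoiding per-second replication.
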(event Custom|StartTimer
  (bind _returnvalue (Utilities|Time|SetTimerbyFunctionName 0 "IncreaseCounter" 1.0 true))
  (Variables|Default|SetTimerHandlerCounter _returnvalue))

(event EventBeginPlay)

(fn ConstructionScript)

(fn IncreaseCounter
  (bind _result (Math|Integer|DecrementInt (Variables|Default|GetTimeCounter))
    (:%20%20
      (Development|PrintString (Utilities|String|ToString(Integer) (stale _result)))
      (Networking|SwitchHasAuthority
        (:Authority
          (if (== (Math|Integer|%(Integer) _result 10) 9)
            (Variables|Default|SetTimeChecker (Variables|Default|GetTimeCounter))
            (CallFunction|SetCounter)
            (else
              (CallFunction|SetCounter))))
        (:Remote
          (CallFunction|SetCounter))))))

(fn OnRepTimeChecker
  (if (!= (Variables|Default|GetTimeChecker) (Variables|Default|GetTimeCounter))
    (Variables|Default|SetTimeCounter (Variables|Default|GetTimeChecker))
    (Utilities|Time|ClearandInvalidateTimerbyHandle (Variables|Default|GetTimerHandlerCounter))
    (bind _returnvalue (Utilities|Time|SetTimerbyFunctionName 0 "IncreaseCounter" 1.0 true))
    (Variables|Default|SetTimerHandlerCounter _returnvalue)
    (CallFunction|SetCounter)))

(fn SetCounter
  (bind _returnvalue (Game|GetPlayerController 0))
  (bind _returnvalue_2 (Pawn|GetControlledPawn _returnvalue))
  (Utilities|IsValid (Variables|Default|GetPlayerCharacter)
    (:Is%20Valid
      _)
    (:Is%20Not%20Valid
      (Utilities|IsValid _returnvalue_2
        (:Is%20Valid
          (bind _asplayer_character (Utilities|Casting|CastToPlayerCharacter _returnvalue_2))
          (Variables|Default|SetPlayerCharacter _asplayer_character)))))
  (Utilities|IsValid (Variables|/Game/Blueprints/Player/Character/PlayerCharacter.PlayerCharacter_C|GetTimerDisplay (Variables|Default|GetPlayerCharacter))
    (:Is%20Valid
      (Default|UpdateTime (Variables|/Game/Blueprints/Player/Character/PlayerCharacter.PlayerCharacter_C|GetTimerDisplay (Variables|Default|GetPlayerCharacter)) (Variables|Default|GetTimeCounter)))))