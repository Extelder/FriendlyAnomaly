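; PlayerCharacter is the player-controlled character Blueprint, handling basic movement, mouse look and jumping.
; Horizontal and Vertical axes move it along the actor's right and forward vectors, and the Jump action's press triggers Jump.
; Mouse axes drive controller yaw and pitch, scaled by a shared Sensetivity variable, with pitch negated.
; BeginPlay sets player controller 0 to game-only input mode.
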(event EventBeginPlay
  (Input|SetInputModeGameOnly (Game|GetPlayerController 0) false))

(event Input|ActionEvents|InputActionJump
  (params (Key :type Key%20Structure :default "None"))
  (:Pressed
    (Character|Jump)))

(event Input|AxisEvents|InputAxishORIZONTAL
  (params (AxisValue :type Float%20%28single-precision%29))
  (Pawn|Input|AddMovementInput (Transformation|GetActorRightVector) AxisValue false))

(event Input|AxisEvents|InputAxisVertical
  (params (AxisValue :type Float%20%28single-precision%29))
  (Pawn|Input|AddMovementInput (Transformation|GetActorForwardVector) AxisValue false))

(event Input|MouseEvents|MouseX
  (params (AxisValue :type Float%20%28single-precision%29))
  (Pawn|Input|AddControllerYawInput (* AxisValue (Variables|Default|GetSensetivity))))

(event Input|MouseEvents|MouseY
  (params (AxisValue :type Float%20%28single-precision%29))
  (Pawn|Input|AddControllerPitchInput (* AxisValue (* -1.0 (Variables|Default|GetSensetivity)))))

(fn ConstructionScript)