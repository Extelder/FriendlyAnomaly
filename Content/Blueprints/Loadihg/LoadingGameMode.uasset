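; LoadingGameMode is a game mode that relays player logins and logouts to the PlayerGameInstance.
; PostLogin and OnLogout feed one shared event, switched by an Add flag.
; Logins add unseen controllers to Players and call NewPlayerLogin, while logouts pass the player state's unique ID to NewPlayerOnLogout without removing the Players entry.
; The similarly named RunOnServerPostLogin function is empty.
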(event Custom|RunOnServerPostLogin1
  (params (PlayerController :type Player%20Controller%20Object%20Reference) (Add :type Boolean) (NetID :type Unique%20Net%20Id%20Repl%20Structure))
  (bind _players (Variables|Default|GetPlayers))
  (if Add
    (if (not (Utilities|Array|ContainsItem _players PlayerController))
      (Utilities|Array|Add _players PlayerController)
      (bind _asplayer_game_instance (Utilities|Casting|CastToPlayerGameInstance (Game|GetGameInstance)))
      (Default|NewPlayerLogin _asplayer_game_instance PlayerController))
    (else
      (bind _asplayer_game_instance_2 (Utilities|Casting|CastToPlayerGameInstance (Game|GetGameInstance)))
      (Default|NewPlayeronLogout _asplayer_game_instance_2 NetID))))

(event EventPostLogin
  (params (NewPlayer :type Player%20Controller%20Object%20Reference))
  (CallFunction|RunonServerPostLogin1 NewPlayer true))

(event EventOnLogout
  (params (ExitingController :type Controller%20Object%20Reference))
  (CallFunction|RunonServerPostLogin1 0 false (PlayerState|GetUniqueID (Variables|/Script/Engine.Controller|GetPlayerState ExitingController))))

(fn ConstructionScript)

(fn RunonServerPostLogin
  (params (PlayerController1 :type Player%20Controller%20Object%20Reference)))