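; Platform lamp light actor with fade-on and fade-off events and a random chance to start as a faulty, flickering lamp.
; On BeginPlay, roughly one in ten lamps calls OffLight, plays a lamp sound and starts LightAnomaly, a self-retriggering loop randomizing intensity and radius.
; OnLight and OffLight lerp PointLight intensity through timelines and set the lamp mesh to its base material, toggling that material's emissive area-lighting flag.
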(event Custom|OffLight
  (bind _sm_platformlamp03 (Variables|Default|GetSM_PlatformLamp03))
  (Variables|Default|SetOnLightBool false)
  (bind _returnvalue (Rendering|Material|CreateDynamicMaterialInstance (Rendering|Material|GetMaterial _sm_platformlamp03 0) "None" "None" :!class /Script/Engine.KismetMaterialLibrary))
  (bind _returnvalue_2 (Rendering|Material|GetBaseMaterial _returnvalue))
  (Variables|/Script/Engine.Material|SetbUseEmissiveForDynamicAreaLighting _returnvalue_2 false)
  (bind _newtrack_0 (Timeline|Timeline PlayFromStart)
    (:Update
      (Rendering|Components|Light|SetIntensity (Variables|Default|GetPointLight) (Math|Float|Lerp 8e+01 0.0 _newtrack_0))
      (Utilities|FlowControl|DoOnce false :!label _label
        (:Completed
          (if (<= _newtrack_0 0.4)
            (Rendering|Material|SetMaterial _sm_platformlamp03 0 _returnvalue_2)
            (else
              (goto _label Reset))))))))

(event Custom|OnLight
  (bind _sm_platformlamp03 (Variables|Default|GetSM_PlatformLamp03))
  (Variables|Default|SetOnLightBool true)
  (bind _returnvalue (Rendering|Material|CreateDynamicMaterialInstance (Rendering|Material|GetMaterial _sm_platformlamp03 0) "None" "None" :!class /Script/Engine.KismetMaterialLibrary))
  (bind _returnvalue_2 (Rendering|Material|GetBaseMaterial _returnvalue))
  (Variables|/Script/Engine.Material|SetbUseEmissiveForDynamicAreaLighting _returnvalue_2 true)
  (Rendering|Material|SetMaterial _sm_platformlamp03 0 _returnvalue_2)
  (bind _newtrack_0 (Timeline|Timeline_0 PlayFromStart)
    (:Update
      (Rendering|Components|Light|SetIntensity (Variables|Default|GetPointLight) (Math|Float|Lerp 0.0 8e+01 _newtrack_0)))))

(event Custom|LightAnomaly
  (Rendering|Components|Light|SetIntensity (Variables|Default|GetPointLight) (Math|Random|RandomFloatinRange 3.0 56.0))
  (Rendering|Lighting|SetAttenuationRadius (Variables|Default|GetPointLight) (Math|Random|RandomFloatinRange 4e+02 7e+02))
  (Utilities|FlowControl|Delay 0.05)
  (CallFunction|LightAnomaly))

(event EventBeginPlay
  (if (>= (Math|Random|RandomIntegerinRange 1 100) 90)
    (CallFunction|OffLight)
    (Audio|PlaySoundatLocation "/Game/Sound/Lamp/Lamp.Lamp" (Transformation|GetActorLocation) "0, 0, 0" 0.4 1.0 0.0 "/Game/Sound/BoomBox/BoomBox.BoomBox" 0 0 0)
    (CallFunction|LightAnomaly)))

(fn ConstructionScript)