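; BP_EndStation is an interactable end station that passes station-ending requests to the level's BP_MainAnomaly, found at BeginPlay.
; Interacting calls CheckGameTypeEndStation on the player, passing the station and that player.
; Its CheckGameType event stores the character and, unless the Wating flag is set, reads GameplayType from PlayerGameInstance.
; It then calls the anomaly's multicast, choose or single end-station function for Random, Choose Player or Single mode.
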(event Custom|CheckGameType
  (params (Character :type Player%20Character%20Object%20Reference))
  (bind _mainanomaly (Variables|Default|GetMainAnomaly))
  (Variables|Default|SetCharacter Character)
  (if (not (Variables|Default|GetWating))
    (bind _asplayer_game_instance (Utilities|Casting|CastToPlayerGameInstance (Game|GetGameInstance)))
    (switch Utilities|FlowControl|Switch|SwitchonPlayerType (Variables|/Game/Blueprints/Player/PlayerGameInstance.PlayerGameInstance_C|GetGameplayType _asplayer_game_instance)
      (:NewEnumerator0
        (Default|EndStationMulticast _mainanomaly (Variables|Default|GetCharacter)))
      (:NewEnumerator1
        (Default|EndStationChoose _mainanomaly (Variables|Default|GetCharacter)))
      (:NewEnumerator2
        (Default|EndStation _mainanomaly)))))

(event EventBeginPlay
  (bind _outactors (Actor|GetAllActorsOfClass "/Game/Blueprints/BP_MainAnomaly.BP_MainAnomaly_C"))
  (Variables|Default|SetMainAnomaly (Utilities|Array|Get(acopy) _outactors)))

(event EventInteractableInteract
  (params (Player :type Player%20Character%20Object%20Reference))
  (Utilities|IsValid Player
    (:Is%20Valid
      (Default|CheckGameTypeEndStation Player self Player))))

(fn ConstructionScript)