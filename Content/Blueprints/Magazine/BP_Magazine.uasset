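; BP_Magazine is an interactable shop Blueprint that holds a money balance and dispatches purchases to buyable components.
; Interacting calls OnMagazine on the player to switch the shop on.
; BalanceAdd raises the balance, while Buy deducts the given amount without an affordability check.
; Buy then loops over the buyable component array and calls OnBuy with the player on valid entries matching the ID.
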(event Custom|Buy
  (params (ID :type Integer) (Type :type BuyEnum%20Enum :default "NewEnumerator0") (Player :type Player%20Character%20Object%20Reference) (Money :type Integer))
  (Variables|Default|SetBalance (- (Variables|Default|GetBalance) Money))
  (switch Utilities|FlowControl|Switch|SwitchonBuyEnum Type
    (:NewEnumerator0
      (for _array_element (Variables|Default|GetBuyableBaseComponent)
        (Utilities|IsValid _array_element
          (:Is%20Valid
            (if (== ID (Variables|/Game/Blueprints/Magazine/Components/BuyableBaseComponent.BuyableBaseComponent_C|GetID _array_element))
              (Default|OnBuy _array_element Player))))))))

(event Custom|BalanceAdd
  (params (Money+ :type Integer))
  (Variables|Default|SetBalance (+ (Variables|Default|GetBalance) Money+)))

(event EventInteractableInteract
  (params (Player :type Player%20Character%20Object%20Reference))
  (Default|OnMagazine Player true false))

(fn ConstructionScript)