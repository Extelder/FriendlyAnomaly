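; Train actor that slides its two doors and travels along X between fixed points, with 2D sounds.
; Chained timelines drive three sequences: full round trip, one-way departure (StartTrainReverse), and delayed arrival (StartTrainOnStart).
; Net update frequency rises for each run and drops when it ends, limiting replication cost.
; While Waiting, a box overlap asks MainAnomaly to count users aboard; BeginPlay gathers four scene components into SceneMassive.
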(event OnComponentBeginOverlap(Box)
  (params (OverlappedComponent :type Primitive%20Component%20Object%20Reference) (OtherActor :type Actor%20Object%20Reference) (OtherComp :type Primitive%20Component%20Object%20Reference) (OtherBodyIndex :type Integer) (bFromSweep :type Boolean) (SweepResult :type Hit%20Result%20Structure%20%28by%20ref%29))
  (if (Variables|Default|GetWaiting)
    (Default|UsersinTrainCount (Variables|Default|GetMainAnomaly))))

(event Custom|StartTrain
  (Variables|Default|SetNetUpdateFrequency 6e+01)
  (Variables|Default|SetMinNetUpdateFrequency 25.0)
  (Audio|PlaySound2D "/Game/Sound/Train/TrainOpenDoor.TrainOpenDoor" 1.0 1.0 0.0 0 0)
  (bind _newtrack_0 (Timeline|DoorOpen PlayFromStart)
    (:Update
      (Transformation|SetRelativeLocation (Variables|Default|GetSM_door_wall_01) (Math|Vector|MakeVector -192.0 (Math|Float|Lerp -158.999998 -214.999998 _newtrack_0) 0.0) false false)
      (Transformation|SetRelativeLocation (Variables|Default|GetSM_door_wall_02) (Math|Vector|MakeVector -192.0 (Math|Float|Lerp -415.999998 -362.999998 _newtrack_0) 0.0) false false))
    (:Finished
      (Audio|PlaySound2D "/Game/Sound/Train/TrainFull.TrainFull" 1.0 1.0 0.0 0 0)
      (bind _newtrack_0_2 (Timeline|Timeline PlayFromStart)
        (:Update
          (Transformation|SetActorLocation (Math|Vector|MakeVector (Math|Float|Lerp 3208.0 -4e+03 _newtrack_0_2) -203.0 1274.0) true false))
        (:Finished
          (Utilities|FlowControl|Delay 4.0)
          (bind _newtrack_0_3 (Timeline|Timeline_0 PlayFromStart)
            (:Update
              (Transformation|SetActorLocation (Math|Vector|MakeVector (Math|Float|Lerp -4e+03 3208.0 _newtrack_0_3) -203.0 1274.0) true false))
            (:Finished
              (Utilities|FlowControl|Delay 1.0)
              (Audio|PlaySound2D "/Game/Sound/Train/TrainOpenDoor.TrainOpenDoor" 1.0 1.0 0.0 0 0)
              (bind _newtrack_0_4 (Timeline|Timeline_1 PlayFromStart)
                (:Update
                  (Transformation|SetRelativeLocation (Variables|Default|GetSM_door_wall_01) (Math|Vector|MakeVector -192.0 (Math|Float|Lerp -214.999998 -158.999998 _newtrack_0_4) 0.0) false false)
                  (Transformation|SetRelativeLocation (Variables|Default|GetSM_door_wall_02) (Math|Vector|MakeVector -192.0 (Math|Float|Lerp -362.999998 -415.999998 _newtrack_0_4) 0.0) false false)
                  (Variables|Default|SetNetUpdateFrequency 5.0)
                  (Variables|Default|SetMinNetUpdateFrequency 5.0))))))))))

(event Custom|StartTrainReverse
  (Variables|Default|SetOnStation? false)
  (Variables|Default|SetNetUpdateFrequency 6e+01)
  (Variables|Default|SetMinNetUpdateFrequency 25.0)
  (Audio|PlaySound2D "/Game/Sound/Train/TrainOpenDoor.TrainOpenDoor" 1.0 1.0 0.0 0 0)
  (bind _newtrack_0 (Timeline|Timeline_2 PlayFromStart)
    (:Update
      (Transformation|SetRelativeLocation (Variables|Default|GetSM_door_wall_01) (Math|Vector|MakeVector -192.0 (Math|Float|Lerp -158.999998 -214.999998 _newtrack_0) 0.0) false false)
      (Transformation|SetRelativeLocation (Variables|Default|GetSM_door_wall_02) (Math|Vector|MakeVector -192.0 (Math|Float|Lerp -415.999998 -362.999998 _newtrack_0) 0.0) false false))
    (:Finished
      (Audio|PlaySound2D "/Game/Sound/Train/TrainReverse.TrainReverse" 1.0 1.0 0.0 0 0)
      (bind _newtrack_0_2 (Timeline|Timeline_3 PlayFromStart)
        (:Update
          (Transformation|SetActorLocation (Math|Vector|MakeVector (Math|Float|Lerp 3208.0 -4e+03 _newtrack_0_2) -203.0 1274.0) true false))
        (:Finished
          (Variables|Default|SetNetUpdateFrequency 5.0)
          (Variables|Default|SetMinNetUpdateFrequency 5.0))))))

(event Custom|StartTrainOnStart
  (Variables|Default|SetOnStation? true)
  (Variables|Default|SetNetUpdateFrequency 6e+01)
  (Variables|Default|SetMinNetUpdateFrequency 25.0)
  (Audio|PlaySound2D "/Game/Sound/Train/TrainStart.TrainStart" 1.0 1.0 0.0 0 0)
  (Utilities|FlowControl|Delay 4.0)
  (bind _newtrack_0 (Timeline|Timeline_0 PlayFromStart)
    (:Update
      (Transformation|SetActorLocation (Math|Vector|MakeVector (Math|Float|Lerp -4e+03 3208.0 _newtrack_0) -203.0 1274.0) true false))
    (:Finished
      (Utilities|FlowControl|Delay 1.0)
      (Audio|PlaySound2D "/Game/Sound/Train/TrainOpenDoor.TrainOpenDoor" 1.0 1.0 0.0 0 0)
      (bind _newtrack_0_2 (Timeline|Timeline_1 PlayFromStart)
        (:Update
          (Transformation|SetRelativeLocation (Variables|Default|GetSM_door_wall_01) (Math|Vector|MakeVector -192.0 (Math|Float|Lerp -214.999998 -158.999998 _newtrack_0_2) 0.0) false false)
          (Transformation|SetRelativeLocation (Variables|Default|GetSM_door_wall_02) (Math|Vector|MakeVector -192.0 (Math|Float|Lerp -362.999998 -415.999998 _newtrack_0_2) 0.0) false false)
          (Variables|Default|SetNetUpdateFrequency 5.0)
          (Variables|Default|SetMinNetUpdateFrequency 5.0))))))

(event EventBeginPlay
  (bind _scenemassive (Variables|Default|GetSceneMassive))
  (Utilities|Array|Add _scenemassive (Variables|Default|GetScene))
  (Utilities|Array|Add _scenemassive (Variables|Default|GetScene1))
  (Utilities|Array|Add _scenemassive (Variables|Default|GetScene2))
  (Utilities|Array|Add _scenemassive (Variables|Default|GetScene3)))

(fn ConstructionScript)