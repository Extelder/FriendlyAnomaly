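; Train actor that, shortly after BeginPlay, pulls into a station and opens its doors.
; A timeline lerps the root 5000 units back along X on fixed Y and Z, spawning a limited number of spark emitters en route.
; After arrival, a second timeline slides six door meshes open.
; The close-doors, depart and repeat chain is disconnected, so the train stays put.
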(event Custom|TrainOutStation
  (bind _newtrack_0 (Timeline|OpenDoor PlayFromStart)
    (:Update
      (Transformation|SetRelativeLocation (Variables|Default|GetSM_door_wall_06) (Math|Vector|MakeVector -193.000025 (Math|Float|Lerp -1543.999998 -1609.999998 _newtrack_0) 0.0) false false)
      (Transformation|SetRelativeLocation (Variables|Default|GetSM_door_wall_05) (Math|Vector|MakeVector -193.000025 (Math|Float|Lerp -1397.999998 -1332.999998 _newtrack_0) 0.0) false false)
      (Transformation|SetRelativeLocation (Variables|Default|GetSM_door_wall_04) (Math|Vector|MakeVector -193.000025 (Math|Float|Lerp -950.999998 -1016.999998 _newtrack_0) 0.0) false false)
      (Transformation|SetRelativeLocation (Variables|Default|GetSM_door_wall_03) (Math|Vector|MakeVector -193.000025 (Math|Float|Lerp -804.999998 -738.0 _newtrack_0) 0.0) false false)
      (Transformation|SetRelativeLocation (Variables|Default|GetSM_door_wall_02) (Math|Vector|MakeVector -193.000025 (Math|Float|Lerp -359.999998 -424.999998 _newtrack_0) 0.0) false false)
      (Transformation|SetRelativeLocation (Variables|Default|GetSM_door_wall_01) (Math|Vector|MakeVector -193.000025 (Math|Float|Lerp -214.999998 -154.999998 _newtrack_0) 0.0) false false))))

(event Custom|TrainToStation
  (Utilities|FlowControl|Delay 5.0)
  (bind _newtrack_0 (Timeline|Timeline PlayFromStart)
    (:Update
      (Transformation|SetWorldLocation (Variables|Default|GetDefaultSceneRoot) (Math|Vector|MakeVector (Math|Float|Lerp (Variables|Default|GetX) (Variables|Default|GetXSubtract) _newtrack_0) -205.0 1272.0) false false)
      (Utilities|FlowControl|Delay 0.2)
      (Utilities|FlowControl|DoN 15
        (:Exit
          (Effects|SpawnEmitteratLocation "/Game/Subway/Particles/PS_Sparks.PS_Sparks" (Transformation|GetWorldLocation (Variables|Default|GetScene))))))
    (:Finished
      (Utilities|FlowControl|Delay 1.0)
      (CallFunction|TrainOutStation))))

(event EventBeginPlay
  (CallFunction|TraintoStation)
  (Variables|Default|SetX (.x (Transformation|GetWorldLocation (Variables|Default|GetDefaultSceneRoot))))
  (Variables|Default|SetXSubtract (- (Variables|Default|GetX) 5e+03)))

(fn ConstructionScript)