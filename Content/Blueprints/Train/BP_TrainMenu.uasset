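; BP_TrainMenu is a train actor, apparently for the menu, that slides along X to a station stop and onward.
; Two timelines lerp the root's location with Y and Z fixed, chained through Finished events and delays into an endless arrive-depart loop that snaps back to the start.
; BeginPlay is empty; the loop's kickoff and X-position setup are disconnected, so nothing in this Blueprint starts the motion.
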(event Custom|TrainOutStation
  (Utilities|FlowControl|Delay 3.0)
  (bind _newtrack_0 (Timeline|Timeline PlayFromStart)
    (:Update
      (Transformation|SetWorldLocation (Variables|Default|GetDefaultSceneRoot) (Math|Vector|MakeVector (Math|Float|Lerp (Variables|Default|GetXSubtract) (* (Variables|Default|GetX) -1.0) _newtrack_0) -205.0 1272.0) false false))
    (:Finished
      (CallFunction|TraintoStation))))

(event Custom|TrainToStation
  (Utilities|FlowControl|Delay 0.5)
  (bind _newtrack_0 (Timeline|TrainAnimation PlayFromStart)
    (:Update
      (Transformation|SetWorldLocation (Variables|Default|GetDefaultSceneRoot) (Math|Vector|MakeVector (Math|Float|Lerp (Variables|Default|GetX) (Variables|Default|GetXSubtract) _newtrack_0) -205.0 1272.0) false false))
    (:Finished
      (CallFunction|TrainOutStation))))

(event EventBeginPlay)

(fn ConstructionScript)