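; BP_Signs02 is a subway sign prop on two cables and two physics constraints that can start with either side broken loose.
; The construction script picks one of three sign meshes from SignsVar.
; On BeginPlay, each enabled break flag detaches that cable's end and breaks its matching constraint.
; The sign then always receives a fixed impulse, whether or not a constraint is broken.
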(event EventBeginPlay
  ;[1 1 1] Break Constraint
  (if (Variables|Default|GetBreak%20Constraint%201)
    (Variables|/Script/CableComponent.CableComponent|SetbAttachEnd (Variables|Default|GetCable1) false)
    (Class|PhysicsConstraintComponent|BreakConstraint (Variables|Components|GetConstL1)))
  (if (Variables|Default|GetBreak%20Constraint%202)
    (Variables|/Script/CableComponent.CableComponent|SetbAttachEnd (Variables|Default|GetCable2) false)
    (Class|PhysicsConstraintComponent|BreakConstraint (Variables|Components|GetConstL2)))
  (Physics|AddImpulse (Variables|Components|GetSigns) "1000.000000,1000.000000,1000.000000" "None" false))

(fn ConstructionScript
  (bind _signs (Variables|Components|GetSigns))
  ;[1 1 1] Mesh Variant
  (switch int (Variables|Default|GetSigns%20Var)
    (:0
      (Components|StaticMesh|SetStaticMesh _signs "/Game/Subway/Meshes/Platform/Signs/SM_Signs04.SM_Signs04"))
    (:1
      (Components|StaticMesh|SetStaticMesh _signs "/Game/Subway/Meshes/Platform/Signs/SM_Signs05.SM_Signs05"))
    (:2
      (Components|StaticMesh|SetStaticMesh _signs "/Game/Subway/Meshes/Platform/Signs/SM_Signs06.SM_Signs06"))))