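; Spline-driven wire Blueprint for the Subway content that builds a cable from spline mesh components in its Construction Script.
; SplineMeshVar places segments either between spline points or at a fixed Spacing along the length, using scaled direction tangents.
; WireVar picks one of six spline mesh component variants, each scaled uniformly by WireSize.
; Two dynamic MI_Wire instances take color, dirt, specular and roughness settings, with TextureVar choosing the texture set.
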(fn ConstructionScript
  (|Wire))