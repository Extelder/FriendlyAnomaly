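; BP_Rails is a subway rail Blueprint that lays spline mesh segments along a spline.
; Its construction script divides the spline length by Spacing and adds one component per step, with RailVar choosing between three spline mesh variants.
; Each segment takes its start and end positions from distances along the spline in local space, with tangents from spline direction scaled by TangentScale.
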(fn ConstructionScript
  (bind _tangent_scale (Variables|Default|GetTangent%20Scale))
  (bind _spline (Variables|Default|GetSpline))
  (bind _spacing (Variables|Default|GetSpacing))
  (Variables|Default|SetComponent%201 0)
  ;[1 1 1] Spline Point Position
  (for _index (range 0 (.ReturnValue (Math|Float|Division(WholeandRemainder) (Spline|GetSplineLength _spline) _spacing)))
    ;[1 1 1] Mesh Variant
    (switch int (Variables|Default|GetRail%20Var)
      (:Default
        (bind _returnvalue (AddComponent|AddSplineMeshComponent false :!label _label))
        (Variables|Default|SetComponent%201 _returnvalue))
      (:0
        (goto _label))
      (:1
        (bind _returnvalue_2 (AddComponent|AddSplineMeshComponent false))
        (Variables|Default|SetComponent%201 _returnvalue_2))
      (:2
        (bind _returnvalue_3 (AddComponent|AddSplineMeshComponent false))
        (Variables|Default|SetComponent%201 _returnvalue_3)))
    (SplineMesh|SetStartandEnd (Variables|Default|GetComponent%201) (Spline|GetLocationatDistanceAlongSpline _spline (* _index _spacing) "Local") (* (Spline|GetDirectionatDistanceAlongSpline _spline (* _index _spacing) "Local") _tangent_scale) (Spline|GetLocationatDistanceAlongSpline _spline (+ (* _index _spacing) _spacing) "Local") (* (Spline|GetDirectionatDistanceAlongSpline _spline (+ (* _index _spacing) _spacing) "Local") _tangent_scale) true :!class /Script/Engine.SplineMeshComponent)))